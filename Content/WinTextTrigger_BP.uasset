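; WinTextTrigger_BP is a trigger actor that fades an orange win-text widget in and out as actors overlap it.
; BeginPlay creates and stores the WinTextWidget.
; Any overlap plays the TextOpacity timeline, which drives the widget's alpha, and ending the overlap reverses it.
; The SetVisibility and AddToViewport calls are disconnected, so this Blueprint never puts the widget on screen.
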(event `self.ReceiveBeginPlay`
  (bind _returnvalue (`|CreateWidget` "/Game/WinTextWidget.WinTextWidget_C"))
  (bind _output_get (set `self.WinTextWidget` _returnvalue)))

(event `self.ReceiveActorBeginOverlap`
  (params (OtherActor :type "Actor Object Reference"))
  (`/Engine/EditorBlueprintResources/StandardMacros.IsValid` (`self.WinTextWidget`)
    (:`Is Valid`
      (bind (_direction _textopacity) (`Timeline|TextOpacity` :!label _label)
        (:`Update`
          (`UserWidget.SetColorAndOpacity` (`self.WinTextWidget`) (`KismetMathLibrary.MakeColor` 1.0 0.56 0.0 _textopacity)))))))

(event `self.ReceiveActorEndOverlap`
  (params (OtherActor :type "Actor Object Reference"))
  (`/Engine/EditorBlueprintResources/StandardMacros.IsValid` (`self.WinTextWidget`)
    (:`Is Valid`
      (goto _label :!via `Reverse`))))

(fn `UserConstructionScript`)