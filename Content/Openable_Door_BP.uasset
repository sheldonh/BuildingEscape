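; Openable door actor that swings open and closed in response to events from its OpenDoor component.
; OnOpen plays the DoorSwing timeline, applying its yaw angle on top of the rotation cached at BeginPlay; OnClose reverses it.
; A timeline event track times a randomly pitched lock sound.
; OnRight and OnWrong play distinct spatialized blips as feedback.
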(event `self.ReceiveBeginPlay`
  (set `self.Initial Rotation` (`self.K2_GetActorRotation`))
  (set `self.Location` (`self.K2_GetActorLocation`)))

(event `self.OpenDoor.OnOpen`
  (bind (_direction _openangle) (`Timeline|Door Swing` :!label _label)
    (:`Update`
      (`self.K2_SetActorRotation` (`KismetMathLibrary.ComposeRotators` (`self.Initial Rotation`) (`KismetMathLibrary.MakeRotator` 0.0 0.0 _openangle))))
    (:`Sound Timing`
      (`GameplayStatics.PlaySoundAtLocation` "/Game/Audio/door-lock.door-lock" (`self.Location`) (struct) 1.0 (`KismetMathLibrary.RandomFloatInRange` 0.8 1.2) 0.0 "/Game/Audio/SpacialAttenuation.SpacialAttenuation"))))

(event `self.OpenDoor.OnClose`
  (goto _label :!via `Reverse`))

(event `self.OpenDoor.OnRight`
  (`GameplayStatics.PlaySoundAtLocation` "/Game/Audio/blip.blip" (`self.Location`) (struct) 0.5 1.0 0.0 "/Game/Audio/SpacialAttenuation.SpacialAttenuation"))

(event `self.OpenDoor.OnWrong`
  (`GameplayStatics.PlaySoundAtLocation` "/Game/Audio/blip2.blip2" (`self.Location`) (struct) 0.3 0.8 0.0 "/Game/Audio/SpacialAttenuation.SpacialAttenuation"))

(fn `UserConstructionScript`)