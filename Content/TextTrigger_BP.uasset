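; Trigger actor that fades an on-screen text widget in when an actor begins overlapping it and out when the overlap ends.
; On BeginPlay it creates the widget, caches its color, adds it to the viewport, and plays or reverses the fade based on player pawn overlap.
; The TextOpacity timeline drives the widget's alpha while keeping its RGB, with no filter on which actor triggers it.
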(event `self.ReceiveActorBeginOverlap`
  (params (OtherActor :type "Actor Object Reference"))
  (bind (_r _g _b) (break `LinearColor` (`self.WidgetColor`)))
  (`/Engine/EditorBlueprintResources/StandardMacros.IsValid` (`self.Widget`)
    (:`Is Valid`
      (bind (_direction _textopacity) (`Timeline|TextOpacity` :!label _label)
        (:`Update`
          (`UserWidget.SetColorAndOpacity` (`self.Widget`) (make `LinearColor` _r _g _b _textopacity)))))))

(event `self.ReceiveBeginPlay`
  (bind _returnvalue (`|CreateWidget` (`self.WidgetClass`)))
  (set `self.Widget` _returnvalue)
  (set `self.WidgetColor` (`UserWidget.ColorAndOpacity` (`self.Widget`)))
  (`Widget.SetVisibility` (`self.Widget`) "Visible")
  (`UserWidget.AddToViewport` (`self.Widget`) 0)
  (if (`self.IsOverlappingActor` (`GameplayStatics.GetPlayerPawn` 0))
    (goto _label)
    (else
      (goto _label :!via `Reverse`))))

(event `self.ReceiveActorEndOverlap`
  (params (OtherActor :type "Actor Object Reference"))
  (`/Engine/EditorBlueprintResources/StandardMacros.IsValid` (`self.Widget`)
    (:`Is Valid`
      (goto _label :!via `Reverse`))))

(fn `UserConstructionScript`)