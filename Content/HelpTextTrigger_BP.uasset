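; HelpTextTrigger_BP is a trigger actor that fades an on-screen help text widget in and out.
; BeginPlay creates a HelpTextWidget, adds it to the viewport and immediately plays the TextOpacity timeline, which drives the alpha of the widget's orange tint.
; Any actor beginning overlap plays the timeline forward and ending overlap reverses it, provided the widget is valid.
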(event `self.ReceiveBeginPlay`
  (bind _returnvalue (`|CreateWidget` "/Game/HelpTextWidget.HelpTextWidget_C"))
  (bind _output_get (set `self.HelpTextWidget` _returnvalue))
  (`Widget.SetVisibility` _output_get "Visible")
  (`UserWidget.AddToViewport` _output_get 0)
  (bind (_direction _textopacity) (`Timeline|TextOpacity` :!label _label)
    (:`Update`
      (`UserWidget.SetColorAndOpacity` (`self.HelpTextWidget`) (`KismetMathLibrary.MakeColor` 1.0 0.56 0.0 _textopacity)))))

(event `self.ReceiveActorBeginOverlap`
  (params (OtherActor :type "Actor Object Reference"))
  (`/Engine/EditorBlueprintResources/StandardMacros.IsValid` (`self.HelpTextWidget`)
    (:`Is Valid`
      (goto _label))))

(event `self.ReceiveActorEndOverlap`
  (params (OtherActor :type "Actor Object Reference"))
  (`/Engine/EditorBlueprintResources/StandardMacros.IsValid` (`self.HelpTextWidget`)
    (:`Is Valid`
      (goto _label :!via `Reverse`))))

(fn `UserConstructionScript`)